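; Test actor for an omni wind field in a Niagara Euler simulation, feeding the player's position to materials and Niagara.
; BeginPlay adds a user interface widget to the viewport.
; Each Tick fills a Vector4 array with index-based placeholder values and prints debug logs.
; While looping over that array, it repeatedly writes the scaled player location to the MPC_WindFiled parameter collection (Z zeroed) and the WindField Niagara variable.
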(event `self.ReceiveBeginPlay`
  (bind _returnvalue (`|CreateWidget` "/Game/NiagaraTest/EulerSimulation/UserInterface.UserInterface_C"))
  (`UserWidget.AddToViewport` _returnvalue 0))

(event `self.ReceiveTick`
  (params (DeltaSeconds :type "Float (single-precision)"))
  (bind _returnvalue (/ (`self.K2_GetActorLocation` (`GameplayStatics.GetPlayerPawn` 0)) 100))
  (bind _returnvalue_2 (`KismetMathLibrary.Conv_VectorToLinearColor` (`KismetMathLibrary.MakeVector` (.x _returnvalue) (.y _returnvalue))))
  (`|ExecutionSequence`
    (:`then_0`
      (`KismetArrayLibrary.Array_Resize` (`self.V4A WindField`) 10))
    (:`then_1`
      (`KismetSystemLibrary.PrintString` "进入循环")
      (for _index (range 11)
        (`KismetSystemLibrary.PrintString` "向数组写入数据")
        (bind _returnvalue_3 (+ _index 0))
        (`KismetArrayLibrary.Array_Set` (`self.V4A WindField`) _index (`KismetMathLibrary.MakeVector4` (`KismetMathLibrary.Conv_IntToDouble` _returnvalue_3) (`KismetMathLibrary.Conv_IntToDouble` _returnvalue_3) (`KismetMathLibrary.Conv_IntToDouble` _returnvalue_3) (`KismetMathLibrary.Conv_IntToDouble` _returnvalue_3)))))
    (:`then_2`
      (`KismetSystemLibrary.PrintString` "读取数组数据")
      (for _array_element (`self.V4A WindField`)
        (`KismetSystemLibrary.PrintString` (`KismetStringLibrary.Conv_VectorToString` (`KismetMathLibrary.Conv_Vector4ToVector` _array_element)))
        (`KismetMaterialLibrary.SetVectorParameterValue` "/Game/NiagaraTest/EulerSimulation/Material/MPC/MPC_WindFiled.MPC_WindFiled" "PlayerPosition" _returnvalue_2)
        (`KismetSystemLibrary.PrintString` (`KismetStringLibrary.Conv_ColorToString` _returnvalue_2))
        (`NiagaraComponent.SetVariableVec3` (`self.WindField`) "PlayerPosition" _returnvalue)))))

(fn `UserConstructionScript`)